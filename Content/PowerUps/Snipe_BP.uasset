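; Sniper weapon power-up Blueprint that fires hitscan shots while the player's Hero wants to shoot, has this power-up active and ammo remains.
; Tick polls those conditions, using a Delay as a makeshift fire-rate limiter flagged for improvement.
; Each shot line-traces from the muzzle socket along camera rotation, plays a sound, decrements ammo and sends DamageMessage to the hit actor.
; Persistent trace drawing and ammo printing provide debug output.
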(event EventTick
  (params (DeltaSeconds :type Float%20%28single-precision%29))
  (bind _staticmesh (Variables|Default|GetStaticMesh))
  (bind _returnvalue (Transformation|GetSocketLocation _staticmesh "Snipe_exit"))
  (bind _ashero (Utilities|Casting|CastToHero (Game|GetPlayerCharacter 0)))
  (if (Variables|/Game/Charater/Hero.Hero_C|GetWants%20to%20shoot _ashero)
    (if (== (Variables|/Game/Charater/Hero.Hero_C|GetPowerUp _ashero) 1)
      (if (>= (Variables|Default|GetSnipe%20Ammo) 1.0)
        ;[1 1 1] Need better Rate of fire
        (Utilities|FlowControl|Delay 0.2)
        (bind _outhit (Collision|LineTraceByChannel _returnvalue (+ _returnvalue (* (Math|Vector|GetForwardVector (Camera|GetCameraRotation (Game|GetPlayerCameraManager 0))) (Variables|Default|GetSnipe%20range))) "TraceTypeQuery1" false 0 "Persistent"))
        (Audio|SpawnSoundatLocation "/Game/StarterContent/Audio/Explosion02.Explosion02" _returnvalue)
        (Development|PrintString (Utilities|String|ToString(Float) (Variables|Default|GetSnipe%20Ammo)) true true "(R=0.655000,G=0.000000,B=0.141858,A=1.000000)")
        (Variables|Default|SetSnipe%20Ammo (- (Variables|Default|GetSnipe%20Ammo) 1.0))
        (Class|ApplyDamage|Damage(Message) (.HitActor (Collision|BreakHitResult _outhit)) (Variables|Default|GetSnipe%20Damage))))))

(fn ConstructionScript)