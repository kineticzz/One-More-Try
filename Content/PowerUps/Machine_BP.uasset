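; Machine gun power-up weapon that fires while the player Hero wants to shoot and has power-up 0 active.
; Tick checks ammo, then uses a Delay to pace automatic fire.
; Each shot line-traces from the M4_exit mesh socket along the camera's forward direction, with debug drawing and an ammo printout.
; It plays an explosion sound, decrements ammo, sends DamageMessage to the hit actor and spawns an emitter at the hit location.
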(event EventTick
  (params (DeltaSeconds :type Float%20%28single-precision%29))
  (bind _staticmesh (Variables|Default|GetStaticMesh))
  (bind _returnvalue (Transformation|GetSocketLocation _staticmesh "M4_exit"))
  ;[1 1 1] Shoot MachineGun
  (bind _ashero (Utilities|Casting|CastToHero (Game|GetPlayerCharacter 0)))
  (if (Variables|/Game/Charater/Hero.Hero_C|GetWants%20to%20shoot _ashero)
    (if (== (Variables|/Game/Charater/Hero.Hero_C|GetPowerUp _ashero) 0)
      (if (>= (Variables|Default|GetM4_ammo) 1.0)
        (Utilities|FlowControl|Delay (Variables|Default|GetM4%20rate))
        (bind _outhit (Collision|LineTraceByChannel _returnvalue (+ _returnvalue (* (Math|Vector|GetForwardVector (Camera|GetCameraRotation (Game|GetPlayerCameraManager 0))) (Variables|Default|GetM4%20Range))) "TraceTypeQuery1" false 0 "ForDuration"))
        (Audio|SpawnSoundatLocation "/Game/StarterContent/Audio/Explosion01.Explosion01" _returnvalue)
        (Development|PrintString (Utilities|String|ToString(Float) (Variables|Default|GetM4_ammo)) true true "(R=0.655000,G=0.000000,B=0.141858,A=1.000000)")
        (Variables|Default|SetM4_ammo (- (Variables|Default|GetM4_ammo) 1.0))
        (Class|ApplyDamage|Damage(Message) (.HitActor (Collision|BreakHitResult _outhit)) (Variables|Default|GetM4_damage))
        (Effects|SpawnEmitteratLocation 0 (.Location (Collision|BreakHitResult _outhit)))))))

(fn ConstructionScript)